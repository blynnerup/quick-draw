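; Samurai duelist in a quick-draw duel, built on a Paper2D sprite and driven by the GM_Duel game mode's phase.
; On BeginPlay it caches the game mode and slides into place with a timeline.
; Attack accepts one press: during Wait it triggers Defeated, during Draw it ends the game and plays a fast lunge timeline.
; That timeline's event track swaps the sprite and reports success, flagging whether the winner is player-controlled.
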(event Custom|SlideIn
  (Components|Timeline|SetPlayRate (Variables|Default|GetSlideInAnim) 2.0)
  (bind _alpha (Timeline|SlideInAnim PlayFromStart)
    (:Update
      (Transformation|SetRelativeLocation (Variables|Default|GetPaperSprite) (Math|Vector|Lerp(Vector) (Variables|Default|GetSlideStartPos) (Variables|Default|GetSpriteDefaultPos) _alpha) false false)
      (CallFunction|SetCrossVisibility false))))

(event Custom|Attack
  (if (not (Variables|Default|GetPressedDraw))
    (switch Utilities|FlowControl|Switch|SwitchonE_Phase (Variables|/Game/Blueprints/GM_Duel.GM_Duel_C|GetPhase (Variables|Default|GetGameMode))
      (:NewEnumerator1
        (CallFunction|SetCrossVisibility true)
        (Variables|Default|SetPressedDraw true)
        (CallFunction|Defeated))
      (:NewEnumerator2
        (Variables|Default|SetPressedDraw true)
        (Default|SetGameFinished (Variables|Default|GetGameMode))
        (Components|Timeline|SetPlayRate (Variables|Default|GetAttackAnim) 8.0)
        (bind _alpha (Timeline|AttackAnim PlayFromStart)
          (:Update
            (Transformation|SetRelativeLocation (Variables|Default|GetPaperSprite) (Math|Vector|Lerp(Vector) (Variables|Default|GetSpriteDefaultPos) (Variables|/Script/Engine.SceneComponent|GetRelativeLocation (Variables|Default|GetAttackPos)) _alpha) false false))
          (:SwitchSprite
            (CallFunction|SetSprite (Variables|Default|GetAttackSprite))
            (Default|AttackSuccess (Variables|Default|GetGameMode) (Pawn|IsPlayerControlled))))))))

(event Custom|Defeated
  (CallFunction|SetSprite (Variables|Default|GetDefeatedSprite))
  (CallFunction|SetCrossVisibility false))

(event EventBeginPlay
  (bind _asgm_duel (Utilities|Casting|CastToGM_Duel (Game|GetGameMode)))
  (Variables|Default|SetGameMode _asgm_duel)
  (Variables|Default|SetSpriteDefaultPos (Variables|/Script/Engine.SceneComponent|GetRelativeLocation (Variables|Default|GetPaperSprite)))
  (CallFunction|Slidein))

(fn ConstructionScript)

(fn SetCrossVisibility
  (params (bNewVisibility :type Boolean))
  (Rendering|SetVisibility (Variables|Default|GetCross) bNewVisibility false))

(fn SetSprite
  (params (NewSprite :type Paper%20Sprite%20Object%20Reference))
  (Rendering|Components|Sprite|SetSprite (Variables|Default|GetPaperSprite) NewSprite)
  ;[1 1 1] This is just in case the sprite renders in a strange way (does not look like in this game)
  (Rendering|Material|SetMaterial (Variables|Default|GetPaperSprite) 0 "/Paper2D/TranslucentUnlitSpriteMaterial.TranslucentUnlitSpriteMaterial")
  (Rendering|SetTranslucentSortPriority (Variables|Default|GetPaperSprite) 1))